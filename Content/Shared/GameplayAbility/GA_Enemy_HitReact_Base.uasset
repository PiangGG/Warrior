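; Base enemy hit-react Gameplay Ability, activated by a gameplay event when an enemy is hit.
; It optionally turns the enemy toward the event instigator, then plays a random montage from its hit-react list.
; A material scalar switches on the hit effect as the montage starts and resets when the ability ends.
; The ability ends when the montage finishes or is interrupted, or after a short delay if no montage is available.
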(event `self.K2_ActivateAbilityFromEvent`
  (params (EventData :type "GameplayEventData Structure (by ref)"))
  (bind _returnvalue (`self.GetEnemyCharacterFromActorInfo`))
  (`|ExecutionSequence`
    (:`then_0`
      (if (`self.FaceAttacker`)
        (`/Engine/EditorBlueprintResources/StandardMacros.IsValid` _returnvalue
          (:`Is Valid`
            (`Actor.K2_SetActorRotation` _returnvalue (`KismetMathLibrary.FindLookAtRotation` (`Actor.K2_GetActorLocation` _returnvalue) (`Actor.K2_GetActorLocation` (`.Instigator` (break `GameplayEventData` EventData)))) false)))))
    (:`then_1`
      (if (`self.HasHitReactMontagesToPlay`)
        (`AbilityTask_PlayMontageAndWait.CreatePlayMontageAndWaitProxy` "None" (`KismetArrayLibrary.Array_Random` (`self.MontagesToPlay`))
          (:`then`
            (`MeshComponent.SetScalarParameterValueOnMaterials` (`self.GetOwningComponentFromActorInfo`) "HitFxSwitch" 1.0)
            (if (not (`self.HasHitReactMontagesToPlay`))
              (`KismetSystemLibrary.Delay` 0.2 :!label _label)
              (`self.K2_EndAbility`)))
          (:`OnCompleted`
            (`self.K2_EndAbility` :!label _label_2))
          (:`OnBlendOut`
            (goto _label_2))
          (:`OnInterrupted`
            (goto _label_2))
          (:`OnCancelled`
            (goto _label_2)))
        (else
          (goto _label))))))

(event `self.K2_OnEndAbility`
  (params (bWasCancelled :type Boolean))
  (`MeshComponent.SetScalarParameterValueOnMaterials` (`self.GetOwningComponentFromActorInfo`) "HitFxSwitch" 0.0))